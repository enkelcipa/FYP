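; Game mode for an office game where the player must finish randomly assigned tasks before the day ends.
; On BeginPlay it caches the player, controller and all BP_BaseTask actors, creates the main HUD and assigns a shuffled subset of roughly a third of the tasks.
; A timeline scaled by DayLength fills the HUD day bar.
; When it finishes, any incomplete assigned task means failure, with win or lose only printed.
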(event Custom|Start%20Day%20Cycle
  (Components|Timeline|SetPlayRate (Variables|Default|GetLerp) (|(1/(Length*60)) (Variables|Default|GetDay%20Length)))
  (bind _alpha (Timeline|Lerp PlayFromStart)
    (:Update
      (Progress|SetPercent (Variables|/Game/Blueprints/UI/WBP_DayTimer.WBP_DayTimer_C|GetDayBar (Variables|/Game/Blueprints/UI/WBP_MainHUD.WBP_MainHUD_C|GetWBP_DayTimer (Variables|References|GetHUD))) (Math|Float|Lerp 0.0 1.0 _alpha)))
    (:Finished
      (CallFunction|DayEnd))))

(event Custom|Create%20HUD
  (bind _returnvalue (UserInterface|CreateWidget "/Game/Blueprints/UI/WBP_MainHUD.WBP_MainHUD_C" (Variables|References|GetPlayer%20Controller)))
  (Variables|References|SetHUD _returnvalue)
  (UserInterface|Viewport|AddtoViewport _returnvalue 0)
  (Variables|/Game/Blueprints/UI/WBP_MainHUD.WBP_MainHUD_C|SetGamemode _returnvalue self)
  (bind _assigned_tasks (CallFunction|GetRandomTasks))
  (Variables|Default|SetAssigned%20Tasks _assigned_tasks)
  (Default|InitialiseMainHUD _returnvalue))

(event Custom|Day%20End
  (bind _array_element (Utilities|Array|ForEachLoopwithBreak (Variables|Default|GetAssigned%20Tasks) :!label _label)
    (:LoopBody
      (if (not (Utilities|Struct|BreakSTaskData (Variables|/Game/Blueprints/Tasks/BP_BaseTask.BP_BaseTask_C|GetTask%20Data _array_element)))
        (CallFunction|FailureState)
        (Variables|Default|SetFailure? true)
        (goto _label Break)))
    (:Completed
      (if (not (Variables|Default|GetFailure?))
        (CallFunction|SuccessState)))))

(event Custom|Failure%20State
  (Development|PrintString "You Lose"))

(event Custom|Init:%20References
  (Utilities|FlowControl|Sequence
    (:then_0
      (bind _returnvalue (Actor|GetActorOfClass "/Game/Blueprints/Char_FirstPerson/BP_FirstPersonCharacter.BP_FirstPersonCharacter_C"))
      (Variables|References|SetPlayer%20Character _returnvalue))
    (:then_1
      (bind _returnvalue_2 (Actor|GetActorOfClass "/Game/Blueprints/Input/BP_FirstPersonPlayerController.BP_FirstPersonPlayerController_C"))
      (Variables|References|SetPlayer%20Controller _returnvalue_2))
    (:then_2
      (bind _outactors (Actor|GetAllActorsOfClass "/Game/Blueprints/Tasks/BP_BaseTask.BP_BaseTask_C"))
      (Variables|Default|SetAll%20Tasks _outactors))))

(event Custom|Success%20State
  (Development|PrintString "You Win"))

(event EventBeginPlay
  (CallFunction|Init:References)
  (CallFunction|CreateHUD)
  (CallFunction|StartDayCycle))

(event EventTaskComplete
  (params (Task%20Object :type BP%20Base%20Task%20Object%20Reference))
  (Default|TaskComplete Task%20Object))

(fn ConstructionScript)

(fn GetRandomTasks
  (Utilities|Array|Clear (LocalVariables|GetTask%20Numbers))
  (Utilities|Array|Clear (LocalVariables|GetTasks%20for%20the%20Day))
  (LocalVariables|SetAmount%20of%20Tasks (Math|Float|Ceil (/ (Utilities|Array|Length (Variables|Default|GetAll%20Tasks)) 3)))
  (for (_ _array_index) (Variables|Default|GetAll%20Tasks)
    (Utilities|Array|Add (LocalVariables|GetTask%20Numbers) _array_index))
  (Utilities|FlowControl|Sequence
    (:then_0
      ;[0.15 0.15 0.15 0.5] Shuffle the Tasks
      (Utilities|Array|Shuffle (LocalVariables|GetTask%20Numbers)))
    (:then_1
      ;[0.15 0.15 0.15 0.5] Get the first 3 items
      (for _index (range 1 (LocalVariables|GetAmount%20of%20Tasks))
        (Utilities|Array|Add (LocalVariables|GetChosen%20Numbers) (Utilities|Array|Get(acopy) (LocalVariables|GetTask%20Numbers) _index))))
    (:then_2
      ;[0.15 0.15 0.15 0.5] Create tasks for the list
      (for _array_element (LocalVariables|GetChosen%20Numbers)
        (Utilities|Struct|SetmembersinSTaskData (Variables|/Game/Blueprints/Tasks/BP_BaseTask.BP_BaseTask_C|GetTask%20Data (Utilities|Array|Get(acopy) (Variables|Default|GetAll%20Tasks) _array_element)) true)
        (Utilities|Array|Add (LocalVariables|GetTasks%20for%20the%20Day) (Utilities|Array|Get(acopy) (Variables|Default|GetAll%20Tasks) _array_element)))
      (return (LocalVariables|GetTasks%20for%20the%20Day)))))
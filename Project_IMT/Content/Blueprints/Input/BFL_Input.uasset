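; Blueprint function library of input and presentation toggles for the first local player.
; Paired functions add or remove Enhanced Input mapping contexts, one pair for basic movement and mouse-look controls and one for task interaction, all at equal priority.
; Other pairs show or hide the mouse cursor and the player character's mesh, leaving child components untouched.
; Each function acts on player index 0 after a validity check.
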(fn `Disable Basic Controls`
  (bind _returnvalue (`GameplayStatics.GetPlayerController` null))
  (bind _returnvalue_2 (pcsubsystem `EnhancedInputLocalPlayerSubsystem` _returnvalue))
  (`/Engine/EditorBlueprintResources/StandardMacros.IsValid` _returnvalue
    (:`Is Valid`
      (`EnhancedInputSubsystemInterface.RemoveMappingContext` _returnvalue_2 "/Game/Blueprints/Input/IMC_Default.IMC_Default" (struct))
      (`EnhancedInputSubsystemInterface.RemoveMappingContext` _returnvalue_2 "/Game/Blueprints/Input/IMC_MouseLook.IMC_MouseLook" (struct)))))

(fn `Disable Task Interaction Controls`
  (bind _returnvalue (`GameplayStatics.GetPlayerController` null))
  (`/Engine/EditorBlueprintResources/StandardMacros.IsValid` _returnvalue
    (:`Is Valid`
      (`EnhancedInputSubsystemInterface.RemoveMappingContext` (pcsubsystem `EnhancedInputLocalPlayerSubsystem` _returnvalue) "/Game/Blueprints/Input/IMC_TaskInteraction.IMC_TaskInteraction" (struct)))))

(fn `Enable Basic Controls`
  (bind _returnvalue (`GameplayStatics.GetPlayerController` null))
  (bind _returnvalue_2 (pcsubsystem `EnhancedInputLocalPlayerSubsystem` _returnvalue))
  (`/Engine/EditorBlueprintResources/StandardMacros.IsValid` _returnvalue
    (:`Is Valid`
      (`EnhancedInputSubsystemInterface.AddMappingContext` _returnvalue_2 "/Game/Blueprints/Input/IMC_Default.IMC_Default" 0 (struct))
      (`EnhancedInputSubsystemInterface.AddMappingContext` _returnvalue_2 "/Game/Blueprints/Input/IMC_MouseLook.IMC_MouseLook" 0 (struct)))))

(fn `Enable Task Interaction Controls`
  (bind _returnvalue (`GameplayStatics.GetPlayerController` null))
  (`/Engine/EditorBlueprintResources/StandardMacros.IsValid` _returnvalue
    (:`Is Valid`
      (`EnhancedInputSubsystemInterface.AddMappingContext` (pcsubsystem `EnhancedInputLocalPlayerSubsystem` _returnvalue) "/Game/Blueprints/Input/IMC_TaskInteraction.IMC_TaskInteraction" 0 (struct)))))

(fn `Hide Cursor`
  (bind _returnvalue (`GameplayStatics.GetPlayerController` null))
  (`/Engine/EditorBlueprintResources/StandardMacros.IsValid` _returnvalue
    (:`Is Valid`
      (set `PlayerController.bShowMouseCursor` false _returnvalue))))

(fn `Hide Player Character`
  (bind _returnvalue (`GameplayStatics.GetPlayerCharacter` null))
  (`/Engine/EditorBlueprintResources/StandardMacros.IsValid` _returnvalue
    (:`Is Valid`
      (`SceneComponent.SetVisibility` (`Character.Mesh` _returnvalue) false false))))

(fn `Show Cursor`
  (bind _returnvalue (`GameplayStatics.GetPlayerController` null))
  (`/Engine/EditorBlueprintResources/StandardMacros.IsValid` _returnvalue
    (:`Is Valid`
      (set `PlayerController.bShowMouseCursor` true _returnvalue))))

(fn `Show Player Character`
  (bind _returnvalue (`GameplayStatics.GetPlayerCharacter` null))
  (`/Engine/EditorBlueprintResources/StandardMacros.IsValid` _returnvalue
    (:`Is Valid`
      (`SceneComponent.SetVisibility` (`Character.Mesh` _returnvalue) true false))))
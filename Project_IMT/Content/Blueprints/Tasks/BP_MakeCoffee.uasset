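; BP_MakeCoffee is a coffee machine task that switches the camera to the machine while active and back to the player on completion.
; On start it spawns a grabbable cup at a random spawn point, destroying it on completion.
; Cursor overlap on the anchor drives cup snapping and unsnapping.
; With a cup placed, one of three buttons sets the widget's coffee strength, marks it poured and shows add-ons.
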(event `self.ReceiveBeginPlay`
  (`parent.ReceiveBeginPlay`)
  (set `self.Anchor Point` (`self.Cup Anchor`)))

(event `self.Task Start`
  (`parent.Task Start`)
  (`PlayerController.SetViewTargetWithBlend` (`GameplayStatics.GetPlayerController` 0) self 1.0 "VTBlend_Linear" 0.0 true)
  (set `self.Started?` true)
  (`self.Spawn Cup`))

(event `self.Task Complete`
  (`PlayerController.SetViewTargetWithBlend` (`GameplayStatics.GetPlayerController` 0) (`GameplayStatics.GetPlayerCharacter` 0) 1.0 "VTBlend_Linear" 0.0 true)
  (set `self.Started?` false)
  (set `self.Poured?` false)
  (set `self.Cup Placed?` false)
  (`self.K2_DestroyActor` (`self.Cup`)))

(event `self.Left Button.OnClicked`
  (params (TouchedComponent :type "PrimitiveComponent Object Reference") (ButtonPressed :type "Key Structure"))
  (if (and (`self.Cup Placed?`) (not (`self.Poured?`)))
    (set `/Game/Blueprints/UI/Tasks/MakeCoffee/WBP_MakeCoffee.Coffee Strength` 1 (`self.Widget`))
    (set `self.Poured?` true :!label _label)
    (`/Game/Blueprints/UI/Tasks/MakeCoffee/WBP_MakeCoffee.Show Addons` (`self.Widget`))))

(event `self.Middle Button.OnClicked`
  (params (TouchedComponent :type "PrimitiveComponent Object Reference") (ButtonPressed :type "Key Structure"))
  (if (and (`self.Cup Placed?`) (not (`self.Poured?`)))
    (set `/Game/Blueprints/UI/Tasks/MakeCoffee/WBP_MakeCoffee.Coffee Strength` 2 (`self.Widget`))
    (goto _label)))

(event `self.Right Button.OnClicked`
  (params (TouchedComponent :type "PrimitiveComponent Object Reference") (ButtonPressed :type "Key Structure"))
  (if (and (`self.Cup Placed?`) (not (`self.Poured?`)))
    (set `/Game/Blueprints/UI/Tasks/MakeCoffee/WBP_MakeCoffee.Coffee Strength` 3 (`self.Widget`))
    (goto _label)))

(event `self.Cup Anchor.OnBeginCursorOver`
  (params (TouchedComponent :type "PrimitiveComponent Object Reference"))
  (bind _cup (`self.Cup`))
  (`/Engine/EditorBlueprintResources/StandardMacros.IsValid` _cup
    (:`Is Valid`
      (if (and (`self.Started?`) (`/Game/Blueprints/Tasks/BP_CoffeeCup.Grabbed?` _cup))
        (`/Game/Blueprints/Tasks/BP_CoffeeCup.Snap to Anchor` (`self.Cup`) (`SceneComponent.K2_GetComponentLocation` (`self.Cup Anchor`)))))))

(event `self.Cup Anchor.OnEndCursorOver`
  (params (TouchedComponent :type "PrimitiveComponent Object Reference"))
  (bind _cup (`self.Cup`))
  (`/Engine/EditorBlueprintResources/StandardMacros.IsValid` _cup
    (:`Is Valid`
      (if (`KismetMathLibrary.BooleanNAND` (`self.Started?`) (`/Game/Blueprints/Tasks/BP_CoffeeCup.Grabbed?` _cup))
        (`/Game/Blueprints/Tasks/BP_CoffeeCup.Unsnap from Anchor` (`self.Cup`))))))

(fn `Spawn Cup`
  (bind _returnvalue (`|SpawnActorFromClass` "/Game/Blueprints/Tasks/BP_CoffeeCup.BP_CoffeeCup_C" (`KismetMathLibrary.MakeTransform` (`SceneComponent.K2_GetComponentLocation` (`KismetArrayLibrary.Array_Random` (`|MakeArray` (`self.Cup Spawn`) (`self.Cup Spawn5`) (`self.Cup Spawn4`) (`self.Cup Spawn3`) (`self.Cup Spawn1`) (`self.Cup Spawn2`))))) "Undefined" "MultiplyWithRoot" null null))
  (bind _output_get (set `self.Cup` _returnvalue))
  (set `/Game/Blueprints/Tasks/BP_CoffeeCup.Coffee Machine` self _output_get))

(fn `UserConstructionScript`
  (`parent.UserConstructionScript`))
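; BP_DiagnoseSystemError is a task Blueprint that drives a timed diagnosis progress bar on a supplied widget.
; StartTimeline stores the widget, scales the Lerp timeline's play rate to the requested seconds and plays it from the start.
; Timeline updates fill the bar from 0 to 1, and completion calls DiagnosisComplete on the widget.
; PauseTimeline and UnpauseTimeline stop and resume the progress, while TaskStart only calls its parent.
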(event `self.Task Start`
  (`parent.Task Start`))

(event `self.Unpause Timeline`
  (bind (_direction _alpha) (`Timeline|Lerp` :!label _label)
    (:`Update`
      (`/Game/Blueprints/UI/Tasks/WBP_DiagnosingSystemError.Fill Progress Bar` (`self.Widget`) (`KismetMathLibrary.Lerp` 0.0 1.0 _alpha)))
    (:`Finished`
      (`/Game/Blueprints/UI/Tasks/WBP_DiagnosingSystemError.Diagnosis Complete` (`self.Widget`)))))

(event `self.Start Timeline`
  (params (`Time in Seconds` :type "Float (double-precision)") (Widget :type "/Game/Blueprints/UI/Tasks/WBP_DiagnosingSystemError Object Reference"))
  (set `self.Widget` Widget)
  (`TimelineComponent.SetPlayRate` (`self.Lerp`) (/ 1.0 `Time in Seconds`))
  (goto _label :!via `PlayFromStart`))

(event `self.Pause Timeline`
  (goto _label :!via `Stop`))

(fn `UserConstructionScript`
  (`parent.UserConstructionScript`))
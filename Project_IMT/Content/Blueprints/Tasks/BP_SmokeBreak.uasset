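; BP_SmokeBreak is a task actor for a smoke break built around a packet of child cigarette actors.
; Starting the task blends the camera to the actor while a timeline lifts and rotates the packet.
; Tagged cigarettes are destroyed in an overlap zone, and destruction events empty the tracked list until the HUD signals completion.
; Completion restores the camera, destroys any grabbed cigarette, reverses the packet and disables the task if none remain.
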(event `self.ReceiveBeginPlay`
  (`parent.ReceiveBeginPlay`)
  (for _array_element (`self.GetAllChildActors` true)
    (bind _asbp_cigarette (cast `/Game/Blueprints/Tasks/BP_Cigarette` _array_element))
    (`KismetArrayLibrary.Array_Add` (`self.Cigarettes`) _asbp_cigarette)
    (set `/Game/Blueprints/Tasks/BP_Cigarette.Smoke Break` self _asbp_cigarette)
    (add `/Game/Blueprints/Tasks/BP_Cigarette.Event: Ciggy Destroyed` _asbp_cigarette (`|CreateDelegate` :!event `Can Continue?`))))

(event `self.Task Start`
  (`parent.Task Start`)
  (`PlayerController.SetViewTargetWithBlend` (`GameplayStatics.GetPlayerController` 0) self 1.0 "VTBlend_Linear" 0.0 true)
  (`self.Move Packet Up`))

(event `Move Packet Up`
  (bind _returnvalue (`SceneComponent.K2_GetComponentLocation` (`self.BaseMesh`)))
  (set `self.Original Position` _returnvalue)
  (set `self.New Position` (`KismetMathLibrary.MakeVector` (.x _returnvalue) (.y _returnvalue) (+ (.z _returnvalue) 10.0)))
  (set `self.Original Rotation` (`SceneComponent.RelativeRotation` (`self.BaseMesh`)))
  (bind (_direction _alpha) (`Timeline|Move Box` :!via `PlayFromStart` :!label _label)
    (:`Update`
      (`SceneComponent.K2_SetWorldLocation` (`self.BaseMesh`) (`KismetMathLibrary.VLerp` (`self.Original Position`) (`self.New Position`) _alpha) false false)
      (`SceneComponent.K2_SetRelativeRotation` (`self.BaseMesh`) (`KismetMathLibrary.RLerp` (`self.Original Rotation`) (struct) _alpha) false false))))

(event `Reset`
  (goto _label :!via `ReverseFromEnd`))

(event `self.Task Complete`
  (bind _returnvalue (`GameplayStatics.GetPlayerController` 0))
  (bind _returnvalue_2 (`GameplayStatics.GetPlayerCharacter` 0))
  (bind _grabbed_cigarette (`self.Grabbed Cigarette`))
  (if (and (`KismetSystemLibrary.IsValid` _returnvalue) (`KismetSystemLibrary.IsValid` _returnvalue_2))
    (`PlayerController.SetViewTargetWithBlend` _returnvalue _returnvalue_2 1.0 "VTBlend_Linear" 0.0 true)
    (`/Engine/EditorBlueprintResources/StandardMacros.IsValid` _grabbed_cigarette
      (:`Is Valid`
        (`self.K2_DestroyActor` _grabbed_cigarette))
      (:`Is Not Valid`
        _))
    (`self.Reset`)
    (if (`KismetArrayLibrary.Array_IsEmpty` (`self.Cigarettes`))
      (`self.Make Unavailable`))))

(event `self.Destroy Ciggy.OnComponentBeginOverlap`
  (params (OverlappedComponent :type "PrimitiveComponent Object Reference") (OtherActor :type "Actor Object Reference") (OtherComp :type "PrimitiveComponent Object Reference") (OtherBodyIndex :type Integer) (bFromSweep :type Boolean) (SweepResult :type "HitResult Structure (by ref)"))
  (if (`self.ActorHasTag` OtherActor "Cig")
    (`self.K2_DestroyActor` OtherActor)))

(event `Can Continue?`
  (params (Ciggy :type "/Game/Blueprints/Tasks/BP_Cigarette Object Reference"))
  (`KismetArrayLibrary.Array_RemoveItem` (`self.Cigarettes`) Ciggy)
  (if (`KismetArrayLibrary.Array_IsEmpty` (`self.Cigarettes`))
    (bind _main_hud (`/Game/Blueprints/BPFL_UsefulFunctions.Get HUD`))
    (message `/Game/Blueprints/Interfaces/BPI_Tasks.Task Complete` _main_hud self)))

(fn `Get Anchor Point`
  (returns (`Anchor Point` :type "ActorComponent Object Reference"))
  (return null))

(fn `UserConstructionScript`
  (`parent.UserConstructionScript`))
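; Draggable coffee cup actor for a coffee machine task, moved with the cursor and snapped into the machine's cup anchor.
; Pickup starts a looping timer and Drop clears it, while Drag follows cursor traces on "Coords"-tagged components in X and Z, locking Y to the machine's anchor.
; Anchor snapping pauses the timer and unsnapping resumes it, with cup placement reported to the coffee machine.
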(event `Find Anchor`
  (bind (_bblockinghit _binitialoverlap _time _distance _location _impactpoint _normal _impactnormal _physmat _hitactor _hitcomponent) (`GameplayStatics.BreakHitResult` (`PlayerController.GetHitResultUnderCursorForObjects` (`GameplayStatics.GetPlayerController` 0) (`|MakeArray` "ObjectTypeQuery8" :!type "EObjectTypeQuery Enum") false)))
  ; Snap to Anchor
  (`/Engine/EditorBlueprintResources/StandardMacros.IsValid` _hitcomponent
    (:`Is Valid`
      (if (`ActorComponent.ComponentHasTag` _hitcomponent "Cup Anchor")
        (`self.K2_SetActorLocation` (`SceneComponent.K2_GetComponentLocation` _hitcomponent))
        (`self.Event: Cup Placed` true)
        (`/Engine/EditorBlueprintResources/StandardMacros.DoOnce` false :!label _label
          (:`Completed`
            (`KismetSystemLibrary.K2_PauseTimerHandle` (`self.Grab Timer`))))))
    (:`Is Not Valid`
      (`KismetSystemLibrary.K2_UnPauseTimerHandle` (`self.Grab Timer`))
      (`self.Event: Cup Placed` false)
      (goto _label :!via `Reset`))))

(event `/Game/Blueprints/Interfaces/BPI_TaskObject.Pickup`
  (bind _returnvalue (`KismetSystemLibrary.K2_SetTimerDelegate` (`|CreateDelegate` :!event `Drag`) 0.01 true))
  (set `self.Grab Timer` _returnvalue))

(event `/Game/Blueprints/Interfaces/BPI_TaskObject.Drop`
  (`KismetSystemLibrary.K2_ClearAndInvalidateTimerHandle` (`self.Grab Timer`))
  (set `self.Grabbed?` false)
  (`self.Reset Grab`))

(event `Drag`
  (bind (_bblockinghit _binitialoverlap _time _distance _location _impactpoint _normal _impactnormal _physmat _hitactor _hitcomponent) (`GameplayStatics.BreakHitResult` (`PlayerController.GetHitResultUnderCursorForObjects` (`GameplayStatics.GetPlayerController` 0) (`|MakeArray` "ObjectTypeQuery8" :!type "EObjectTypeQuery Enum") false)))
  (bind (_returnvalue_x _returnvalue_y) (`KismetMathLibrary.BreakVector` (`SceneComponent.K2_GetComponentLocation` (`/Game/Blueprints/Tasks/BP_MakeCoffee.Anchor Point` (`self.Coffee Machine`)))))
  ; Drag
  (`|ExecutionSequence`
    (:`then_0`
      (`/Engine/EditorBlueprintResources/StandardMacros.DoOnce` false :!label _label_2
        (:`Completed`
          (set `self.Grabbed?` true))))
    (:`then_1`
      (if (`ActorComponent.ComponentHasTag` _hitcomponent "Coords")
        (`self.K2_SetActorLocation` (`KismetMathLibrary.MakeVector` (.x _impactpoint) _returnvalue_y (.z _impactpoint)))))))

(event `Reset Grab`
  ; Drag
  (goto _label_2 :!via `Reset`))

(event `Snap to Anchor`
  (params (Location :type "Vector Structure"))
  (set `self.Anchor Location` Location)
  (set `/Game/Blueprints/Tasks/BP_MakeCoffee.Cup Placed?` true (`self.Coffee Machine`))
  (`KismetSystemLibrary.K2_PauseTimerHandle` (`self.Grab Timer`))
  (`self.K2_SetActorLocation` (`self.Anchor Location`)))

(event `Unsnap from Anchor`
  (`KismetSystemLibrary.K2_UnPauseTimerHandle` (`self.Grab Timer`))
  (if (!= (`self.K2_GetActorLocation`) (`self.Anchor Location`))
    (set `/Game/Blueprints/Tasks/BP_MakeCoffee.Cup Placed?` false (`self.Coffee Machine`))))

(fn `Get Anchor Point`
  (returns (`Anchor Point` :type "ActorComponent Object Reference"))
  (return (`/Game/Blueprints/Tasks/BP_MakeCoffee.Anchor Point` (`self.Coffee Machine`))))

(fn `UserConstructionScript`)
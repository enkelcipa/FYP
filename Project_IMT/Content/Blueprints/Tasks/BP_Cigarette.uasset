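; Grabbable cigarette actor for the SmokeBreak task, dragged with the cursor and then set up for lighting.
; Pickup starts looping timers for dragging, which follows cursor hits on "Coords" components, and falling, which sinks it while not grabbed.
; Overlapping a "Smoke" component drops it, rotates it by timeline, blends the camera to it and hands it to the task widget.
; A separate event rolls the mesh, and EndPlay broadcasts its destruction.
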(event `/Game/Blueprints/Interfaces/BPI_TaskObject.Pickup`
  (set `/Game/Blueprints/Tasks/BP_SmokeBreak.Grabbed Cigarette` self (`self.Smoke Break`))
  (bind _returnvalue (`KismetSystemLibrary.K2_SetTimerDelegate` (`|CreateDelegate` :!event `Drag`) 0.01 true))
  (set `self.Drag Timer` _returnvalue)
  (bind _returnvalue_2 (`KismetSystemLibrary.K2_SetTimerDelegate` (`|CreateDelegate` :!event `Fall`) 0.0005 true))
  (set `self.Drop Timer` _returnvalue_2))

(event `/Game/Blueprints/Interfaces/BPI_TaskObject.Drop`
  (`KismetSystemLibrary.K2_ClearAndInvalidateTimerHandle` (`self.Drag Timer`))
  (set `self.Grabbed?` false)
  (`self.Reset Grab`)
  (set `/Game/Blueprints/Tasks/BP_SmokeBreak.Grabbed Cigarette` null (`self.Smoke Break`)))

(event `Drag`
  (bind (_bblockinghit _binitialoverlap _time _distance _location _impactpoint _normal _impactnormal _physmat _hitactor _hitcomponent) (`GameplayStatics.BreakHitResult` (`PlayerController.GetHitResultUnderCursorForObjects` (`GameplayStatics.GetPlayerController` 0) (`|MakeArray` "ObjectTypeQuery8" :!type "EObjectTypeQuery Enum") false)))
  (`|ExecutionSequence`
    (:`then_0`
      (`/Engine/EditorBlueprintResources/StandardMacros.DoOnce` false :!label _label
        (:`Completed`
          (set `self.Grabbed?` true))))
    (:`then_1`
      (if (`ActorComponent.ComponentHasTag` _hitcomponent "Coords")
        (`self.K2_SetActorLocation` _impactpoint)))))

(event `Reset Grab`
  (goto _label :!via `Reset`))

(event `Fall`
  (bind (_returnvalue_x _returnvalue_y _returnvalue_z) (`KismetMathLibrary.BreakVector` (`self.K2_GetActorLocation`)))
  (if (not (`self.Grabbed?`))
    (`self.K2_SetActorLocation` (`KismetMathLibrary.MakeVector` _returnvalue_x _returnvalue_y (- _returnvalue_z 0.01)))))

(event `self.Box.OnComponentBeginOverlap`
  (params (OverlappedComponent :type "PrimitiveComponent Object Reference") (OtherActor :type "Actor Object Reference") (OtherComp :type "PrimitiveComponent Object Reference") (OtherBodyIndex :type Integer) (bFromSweep :type Boolean) (SweepResult :type "HitResult Structure (by ref)"))
  (if (`ActorComponent.ComponentHasTag` OtherComp "Smoke")
    (`self.Prepare for Lighting`)
    (`self.Drop`)))

(event `Prepare for Lighting`
  (`/Engine/EditorBlueprintResources/StandardMacros.DoOnce` false
    (:`Completed`
      (`KismetSystemLibrary.K2_ClearAndInvalidateTimerHandle` (`self.Drop Timer`))
      (bind _output_get (set `self.Initial Rotation` (`SceneComponent.RelativeRotation` (`self.StaticMesh`))))
      (set `self.New Rotation` (`KismetMathLibrary.MakeRotator` (.roll _output_get) (- (.pitch _output_get) 90.0) (.yaw _output_get)))
      (bind (_direction _alpha) (`Timeline|Rotate Cig` :!via `PlayFromStart`)
        (:`Update`
          (`SceneComponent.K2_SetRelativeRotation` (`self.StaticMesh`) (`KismetMathLibrary.RLerp` (`self.Initial Rotation`) (`self.New Rotation`) _alpha) false false))
        (:`Finished`
          (`PlayerController.SetViewTargetWithBlend` (`GameplayStatics.GetPlayerController` 0) self 1.0 "VTBlend_Linear" 0.0 false)
          (`KismetSystemLibrary.Delay` 1.0)
          (bind _widget (message `/Game/Blueprints/Interfaces/BPI_Tasks.Get Current Task Widget` (`GameplayStatics.GetGameMode`)))
          (message `/Game/Blueprints/Interfaces/BPI_Tasks.Toggle Task Widget Visibility` _widget true)
          (message `/Game/Blueprints/Interfaces/BPI_Tasks.Parse Actor` _widget self)
          (set `/Game/Blueprints/Tasks/BP_SmokeBreak.Grabbed Cigarette` self (`self.Smoke Break`)))))))

(event `/Game/Blueprints/Interfaces/BPI_TaskObject.Rotate Object`
  (bind _output_get (set `self.Initial Rotation` (`SceneComponent.RelativeRotation` (`self.StaticMesh`))))
  (set `self.New Rotation` (`KismetMathLibrary.MakeRotator` (+ (.roll _output_get) 90.0) (.pitch _output_get) (.yaw _output_get)))
  (bind (_direction _alpha) (`Timeline|Timeline` :!via `PlayFromStart`)
    (:`Update`
      (`SceneComponent.K2_SetRelativeRotation` (`self.StaticMesh`) (`KismetMathLibrary.RLerp` (`self.Initial Rotation`) (`self.New Rotation`) _alpha) false false))))

(event `self.ReceiveEndPlay`
  (params (EndPlayReason :type "EEndPlayReason Enum" :default "Destroyed"))
  (`self.Event: Ciggy Destroyed` self))

(fn `Get Anchor Point`
  (returns (`Anchor Point` :type "ActorComponent Object Reference"))
  (return null))

(fn `UserConstructionScript`)
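; BP_BaseTask is the base actor for interactable tasks, tracking availability and completion in its TaskData struct.
; An assigned task becomes available once its spawn time elapses, turning its NSAssignedTask effect green; completion or unavailability deactivates the effect.
; Interacting with an available, incomplete task hides the player, switches from movement to cursor controls and opens the task's widget.
; The timeline start, pause and unpause events are empty stubs.
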(event `self.ReceiveBeginPlay`
  ; Set the Actor in the Struct
  (setmembers `/Game/Blueprints/STaskData` :`StructRef` (`self.Task Data`) :`Task Actor` self))

(event `/Game/Blueprints/Interfaces/BPI_ActorInteract.Interact`
  (params (`Interacting Character` :type "/Game/Blueprints/Char_FirstPerson/BP_FirstPersonCharacter Object Reference"))
  (bind ((`Available?_33_8226BE554A0BE593724E5C89D6E76CEA` _available_) (`Completed?_35_0C5B03E846BFDB29F72849AA4EE91809` _completed_)) (break `/Game/Blueprints/STaskData` (`self.Task Data`)))
  (if (and _available_ (not _completed_))
    (`self.Task Start`)))

(event `Is Available?`
  (bind ((`TimeUntilSpawn_19_E5AF35CE4BEE6F90E4C5FB8980729E51` _timeuntilspawn) (`Assigned?_25_0FE19AAB4C3905094417B8861A8629B2` _assigned_)) (break `/Game/Blueprints/STaskData` (`self.Task Data`)))
  (if (and (<= _timeuntilspawn 0.0) _assigned_)
    (`self.Make Available`)))

(event `Task Start`
  (bind _returnvalue (`GameplayStatics.GetPlayerController` 0))
  (bind ((`TaskActor_26_11E7B66D47B07908900001819C91ECB7` _taskactor) (`TaskWidget_31_B5C0A95A4E526B164AFA0086879ED036` _taskwidget)) (break `/Game/Blueprints/STaskData` (`self.Task Data`)))
  (`/Game/Blueprints/Input/BFL_Input.Disable Basic Controls`)
  (`/Game/Blueprints/Input/BFL_Input.Hide Player Character`)
  (`/Game/Blueprints/Input/BFL_Input.Show Cursor`)
  (`/Game/Blueprints/Input/BFL_Input.Enable Task Interaction Controls`)
  (bind _returnvalue_2 (`|CreateWidget` _taskwidget (`GameplayStatics.GetPlayerController` 0)))
  (`self.Event: Open Task` _returnvalue_2 _taskactor)
  (`Controller.SetIgnoreMoveInput` _returnvalue true)
  (`Controller.SetIgnoreLookInput` _returnvalue true))

(event `Task Complete`
  (setmembers `/Game/Blueprints/STaskData` :`StructRef` (`self.Task Data`) :`Completed?` true)
  (`ActorComponent.Deactivate` (`self.NS_AssignedTask`)))

(event `/Game/Blueprints/Interfaces/BPI_ActorInteract.Make Available`
  (setmembers `/Game/Blueprints/STaskData` :`StructRef` (`self.Task Data`) :`Available?` true)
  (`self.Update Sprite Colour` (struct :`G` 1.0 :`A` 1.0)))

(event `Update Sprite Colour`
  (params (Colour :type "LinearColor Structure"))
  (`FXSystemComponent.SetColorParameter` (`self.NS_AssignedTask`) "Colour" Colour))

(event `/Game/Blueprints/Interfaces/BPI_ActorInteract.Make Unavailable`
  (setmembers `/Game/Blueprints/STaskData` :`StructRef` (`self.Task Data`) :`Available?` false)
  (`ActorComponent.Deactivate` (`self.NS_AssignedTask`)))

(event `Start Timeline`
  (params (`Time in Seconds` :type "Float (double-precision)") (Widget :type "/Game/Blueprints/UI/Tasks/WBP_DiagnosingSystemError Object Reference")))

(event `Pause Timeline`)

(event `Unpause Timeline`)

(fn `UserConstructionScript`)
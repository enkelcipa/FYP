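; Bathroom door actor that swings open and closed on alternate interactions.
; BeginPlay stores the starting rotation, and Interact uses a FlipFlop to play the RotateDoor timeline from the start or reverse it from the end.
; The timeline's Alpha lerps the whole actor's rotation between StartRotation and EndRotation, so an interaction mid-swing snaps to an endpoint first.
; GetCurrentTaskWidget is an empty stub.
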(event `self.ReceiveBeginPlay`
  (set `self.Start Rotation` (`self.K2_GetActorRotation`)))

(event `/Game/Blueprints/Interfaces/BPI_ActorInteract.Interact`
  (params (`Interacting Character` :type "/Game/Blueprints/Char_FirstPerson/BP_FirstPersonCharacter Object Reference"))
  (`/Engine/EditorBlueprintResources/StandardMacros.FlipFlop`
    (:`A`
      (bind (_direction _alpha) (`Timeline|Rotate Door` :!via `PlayFromStart` :!label _label)
        (:`Update`
          (`self.K2_SetActorRotation` (`KismetMathLibrary.RLerp` (`self.Start Rotation`) (`self.End Rotation`) _alpha)))))
    (:`B`
      (goto _label :!via `ReverseFromEnd`))))

(fn `Get Current Task Widget`
  (returns (Widget :type "Widget Object Reference"))
  (return null))

(fn `UserConstructionScript`)